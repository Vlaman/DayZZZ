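; Character health component that tracks current and maximum HP and handles healing with first aid kits.
; BeginPlay seeds MaxHp and NowHp from the Health variable's Health field and the heal amount from its FirstAidKit field.
; UseFirstAidKit spends one kit from a separate FirstAidKit counter, if any remain, and adds the heal amount, capped at MaxHp.
; It contains no damage logic.
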(event `self.ReceiveBeginPlay`
  (bind (_health _firstaidkit) (break `/Game/Characters/BPC/BPC_health/EN_health` (`self.Health`)))
  (set `self.healing` _firstaidkit)
  (set `self.max_hp` _health)
  (bind _output_get (set `self.now_hp` (`.health_5_0C5945AC4E050980239E4388CC9508D7` (break `/Game/Characters/BPC/BPC_health/EN_health` (`self.Health`))))))

(fn `use_first aid kit`
  (bind _returnvalue (+ (`self.now_hp`) (`self.healing`)))
  (if (> (`self.first aid kit`) 0)
    (set `self.first aid kit` (- (`self.first aid kit`) 1))
    (if (> _returnvalue (`self.max_hp`))
      (set `self.now_hp` (- (`self.now_hp`) (- (`self.now_hp`) (`self.max_hp`) 0) 0))
      (else
        (set `self.now_hp` _returnvalue)))
    (return)))